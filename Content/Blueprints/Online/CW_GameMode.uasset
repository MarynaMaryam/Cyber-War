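; Online game mode that respawns players at player starts belonging to their team.
; On login it binds each CW_PlayerController's death event to a respawn, which waits on one shared retriggerable delay, then spawns and possesses a default pawn.
; FindPlayerStart and ChoosePlayerStart overrides randomly pick a CW_PlayerStart matching the player state's Team, falling back to parent logic when none match.
; The random pick never selects the last match when several exist.
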(event Custom|RespawnPlayer
  (params (Player :type CW%20Player%20Controller%20Object%20Reference))
  (Utilities|FlowControl|RetriggerableDelay (Variables|Default|GetMinRespawnDelay))
  (CallFunction|Respawn Player))

(event EventBeginPlay)

(event EventTick
  (params (DeltaSeconds :type Float%20%28single-precision%29)))

(event EventPostLogin
  (params (NewPlayer :type Player%20Controller%20Object%20Reference))
  (bind _ascw_player_controller (Utilities|Casting|CastToCW_PlayerController NewPlayer))
  (EventDispatchers|BindEventtoOnDeathPlayer _ascw_player_controller (delegate Custom|RespawnPlayer)))

(fn ConstructionScript)

(fn Respawn
  (params (Player :type Controller%20Object%20Reference))
  (bind _returnvalue (Game|SpawnActorfromClass (Variables|Default|GetDefaultPawnClass) (Transformation|GetActorTransform (Class|GameModeBase|FindPlayerStart Player)) "AdjustIfPossibleButDontSpawnIfColliding" Player 0))
  (Pawn|Possess Player _returnvalue)
  (return))

(fn GetPlayerStart
  (params (Player :type Controller%20Object%20Reference))
  (bind _playerstarts (LocalVariables|GetPlayerStarts))
  (bind _returnvalue (Utilities|Array|Length _playerstarts))
  (Utilities|Array|Clear (LocalVariables|GetPlayerStarts))
  (bind _ascw_player_controller (Utilities|Casting|CastToCW_PlayerController Player))
  (bind _outactors (Actor|GetAllActorsOfClass "/Game/Blueprints/Game/CW_PlayerStart.CW_PlayerStart_C"))
  (for _array_element _outactors
    (if (Utilities|Enum|Equal(Enum) (Variables|/Game/Blueprints/Game/CW_PlayerStart.CW_PlayerStart_C|GetTeam _array_element) (Variables|/Game/Blueprints/Player/CW_PlayerState.CW_PlayerState_C|GetTeam (.AsCW%20Player%20State (Utilities|Casting|CastToCW_PlayerState (Variables|/Script/Engine.Controller|GetPlayerState _ascw_player_controller)))))
      (Utilities|Array|Add (LocalVariables|GetPlayerStarts) _array_element)))
  (return (Utilities|Array|Get(acopy) _playerstarts (Math|Random|RandomInteger (- _returnvalue 1))) (> _returnvalue 0)))

(fn FindPlayerStart
  (params (Player :type Controller%20Object%20Reference) (IncomingName :type String))
  (bind (_playerstart _success) (CallFunction|GetPlayerStart Player))
  (bind _returnvalue (|CallParentFunction Player IncomingName))
  (return (select _success _playerstart _returnvalue)))

(fn ChoosePlayerStart
  (params (Player :type Controller%20Object%20Reference))
  (bind (_playerstart _success) (CallFunction|GetPlayerStart Player))
  (bind _returnvalue (|CallParentFunction Player))
  (return (select _success _playerstart _returnvalue)))