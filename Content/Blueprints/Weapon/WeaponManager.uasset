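; Weapon inventory component for CW_Character that manages five weapon slots, default spawning, pickup, dropping, selection and forwarding of attack and reload input.
; Capsule overlaps pick up interactable weapons only into empty Primary or Secundary slots, with pickup and single drop sent through multicast events.
; SetWeapon fills slots and triggers selection, which updates Equipping and LastWeapon.
; RepNotifies assign owners, update selected and previous weapons, and fall back when Primary or Secundary empties.
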(event Custom|OnPlayerOverlap
  (params (OverlappedComponent :type Primitive%20Component%20Object%20Reference) (OtherActor :type Actor%20Object%20Reference) (OtherComp :type Primitive%20Component%20Object%20Reference) (OtherBodyIndex :type Integer) (bFromSweep :type Boolean) (SweepResult :type Hit%20Result%20Structure%20%28by%20ref%29))
  (CallFunction|HandleRaise OtherActor))

(event EventBeginPlay
  (bind _ascw_character (Utilities|Casting|CastToCW_Character (Components|GetOwner)))
  (Variables|Default|SetPlayerOwner _ascw_character)
  (Collision|BindEventtoOnComponentBeginOverlap (Variables|/Script/Engine.Character|GetCapsuleComponent (Variables|Default|GetPlayerOwner)) (delegate Custom|OnPlayerOverlap)))

(event EventTick
  (params (DeltaSeconds :type Float%20%28single-precision%29)))

(event Custom|HandleRaise
  (params (Actor :type Actor%20Object%20Reference))
  (bind _asweapon (Utilities|Casting|CastToWeapon Actor))
  (if (Utilities|DoesObjectImplementInterface Actor "/Game/Blueprints/Interface/IE_Interact.IE_Interact_C")
    (if (CallFunction|CanRaiseWeapon (Variables|/Game/Blueprints/Weapon/Weapon.Weapon_C|GetWeaponSlot _asweapon))
      (CallFunction|MulticastRaise _asweapon))))

(event Custom|BaseAttack
  (params (Activated :type Boolean))
  (bind _weapon (CallFunction|GetWeaponSelected))
  (Utilities|IsValid _weapon
    (:Is%20Valid
      (Default|StartAttack _weapon Activated "NewEnumerator0"))))

(event Custom|AdvancedAttack
  (params (Activated :type Boolean))
  (bind _weapon (CallFunction|GetWeaponSelected))
  (Utilities|IsValid _weapon
    (:Is%20Valid
      (Default|StartAttack _weapon Activated "NewEnumerator1"))))

(event Custom|Reloading
  (bind _weapon (CallFunction|GetWeaponSelected))
  (Utilities|IsValid _weapon
    (:Is%20Valid
      (Default|StartReloading _weapon))))

(event Custom|MulticastRaise
  (params (Actor :type Actor%20Object%20Reference))
  (Class|IEInteract|Interact(Message) Actor (Components|GetOwner)))

(event Custom|MulticastDropped
  (params (Weapon :type Weapon%20Object%20Reference))
  (Default|Dropped Weapon))

(fn SpawnWeapon
  (params (Weapon :type Weapon%20Class%20Reference))
  (bind _returnvalue (Components|GetOwner))
  (bind _returnvalue_2 (Game|SpawnActorfromClass Weapon (Transformation|GetActorTransform _returnvalue) "AlwaysSpawn" _returnvalue 0))
  (CallFunction|SetWeapon (Variables|/Game/Blueprints/Weapon/Weapon.Weapon_C|GetWeaponSlot _returnvalue_2) _returnvalue_2))

(fn GetWeaponSelected
  (return (Variables|Default|GetEquipping)))

(fn SetWeapon
  (params (Slot :type EWeaponSlot%20Enum :default "NewEnumerator0") (Weapon :type Weapon%20Object%20Reference))
  (LocalVariables|SetLocalWeapon Weapon)
  (Utilities|FlowControl|Sequence
    (:then_0
      (switch Utilities|FlowControl|Switch|SwitchonEWeaponSlot Slot
        (:NewEnumerator0
          (Variables|Default|SetPrimary (LocalVariables|GetLocalWeapon)))
        (:NewEnumerator1
          (Variables|Default|SetSecundary (LocalVariables|GetLocalWeapon)))
        (:NewEnumerator2
          (Variables|Default|SetMelee (LocalVariables|GetLocalWeapon)))
        (:NewEnumerator3
          (Variables|Default|SetThrow (LocalVariables|GetLocalWeapon)))
        (:NewEnumerator4
          (Variables|Default|SetSpecial (LocalVariables|GetLocalWeapon)))))
    (:then_1
      (Utilities|IsValid (Variables|Default|GetEquipping)
        (:Is%20Valid
          (Utilities|IsValid (LocalVariables|GetLocalWeapon)
            (:Is%20Valid
              (CallFunction|SelectedWeapon (Variables|/Game/Blueprints/Weapon/Weapon.Weapon_C|GetWeaponSlot (LocalVariables|GetLocalWeapon)))
              (return))
            (:Is%20Not%20Valid
              (return))))
        (:Is%20Not%20Valid
          (CallFunction|SelectedWeapon "NewEnumerator2")
          (return))))))

(fn SelectedWeapon
  (params (Slot :type EWeaponSlot%20Enum :default "NewEnumerator0"))
  (if (CallFunction|CanEquippingWeapon Slot)
    (Utilities|IsValid (Variables|Default|GetEquipping)
      (:Is%20Valid
        (Variables|Default|SetLastWeapon (Variables|Default|GetEquipping)))
      (:Is%20Not%20Valid
        _))
    (Variables|Default|SetEquipping (CallFunction|GetWeapon Slot))
    (return)
    (else
      (return))))

(fn CanEquippingWeapon
  (params (Slot :type EWeaponSlot%20Enum :default "NewEnumerator0"))
  (bind _equipping (Variables|Default|GetEquipping))
  (Utilities|IsValid _equipping
    (:Is%20Valid
      (return (and (Utilities|Enum|NotEqual(Enum) Slot (Variables|/Game/Blueprints/Weapon/Weapon.Weapon_C|GetWeaponSlot _equipping)) (Utilities|IsValid (CallFunction|GetWeapon Slot)))))
    (:Is%20Not%20Valid
      (return true))))

(fn GetWeapon
  (params (Slot :type EWeaponSlot%20Enum%20%28by%20ref%29 :default "NewEnumerator0"))
  (return (Utilities|Select :Index Slot :NewEnumerator0 (Variables|Default|GetPrimary) :NewEnumerator1 (Variables|Default|GetSecundary) :NewEnumerator2 (Variables|Default|GetMelee) :NewEnumerator3 (Variables|Default|GetThrow) :NewEnumerator4 (Variables|Default|GetSpecial))))

(fn SpawnDefaultWeapons
  (for _array_element (Variables|Default|GetDefaultsWeapon)
    (CallFunction|SpawnWeapon _array_element))
  (return))

(fn OnRepEquipping
  (bind _equipping (Variables|Default|GetEquipping))
  (Utilities|IsValid _equipping
    (:Is%20Valid
      (Default|SelectedWeapon _equipping)
      (return))
    (:Is%20Not%20Valid
      (return))))

(fn OnRepPrimary
  (bind _primary (Variables|Default|GetPrimary))
  (Utilities|IsValid _primary
    (:Is%20Valid
      (Default|SetOwnerWeapon _primary (Components|GetOwner))
      (return))
    (:Is%20Not%20Valid
      (CallFunction|SelectedBestWeapon)
      (return))))

(fn OnRepSecundary
  (bind _secundary (Variables|Default|GetSecundary))
  (Utilities|IsValid _secundary
    (:Is%20Valid
      (Default|SetOwnerWeapon _secundary (Components|GetOwner))
      (return))
    (:Is%20Not%20Valid
      (CallFunction|SelectedBestWeapon)
      (return))))

(fn OnRepMelee
  (bind _melee (Variables|Default|GetMelee))
  (Utilities|IsValid _melee
    (:Is%20Valid
      (Default|SetOwnerWeapon _melee (Components|GetOwner))
      (return))
    (:Is%20Not%20Valid
      (return))))

(fn OnRepThrow)

(fn OnRepSpecial)

(fn OnRepLastWeapon
  (bind _lastweapon (Variables|Default|GetLastWeapon))
  (Utilities|IsValid _lastweapon
    (:Is%20Valid
      (if (!= (Components|GetOwner _lastweapon) (Components|GetOwner))
        (return)
        (else
          (Default|CaseWeapon _lastweapon)
          (return))))
    (:Is%20Not%20Valid
      (return))))

(fn DroppedWeapon
  (bind _equipping (Variables|Default|GetEquipping))
  (Utilities|IsValid _equipping
    (:Is%20Valid
      (if (Default|CanDroppedWeapon _equipping)
        (CallFunction|MulticastDropped _equipping)
        (CallFunction|SetWeapon (Variables|/Game/Blueprints/Weapon/Weapon.Weapon_C|GetWeaponSlot _equipping))
        (else
          (return))))
    (:Is%20Not%20Valid
      (return))))

(fn CanRaiseWeapon
  (params (Slot :type EWeaponSlot%20Enum :default "NewEnumerator0"))
  (switch Utilities|FlowControl|Switch|SwitchonEWeaponSlot Slot
    (:NewEnumerator0
      (Variables|Default|GetPrimary
        (:then
          _)
        (:else
          (return true))))
    (:NewEnumerator1
      (Variables|Default|GetSecundary
        (:then
          _)
        (:else
          (return true))))
    (:NewEnumerator2
      (return false)))
  (return false))

(fn DroppedAllWeapons
  (bind _melee (Variables|Default|GetMelee))
  (for _array_element (Utilities|Array|MakeArray (Variables|Default|GetPrimary) (Variables|Default|GetSecundary) (Variables|Default|GetSpecial))
    (Utilities|IsValid _array_element
      (:Is%20Valid
        (if (Default|CanDroppedWeapon _array_element)
          (Default|Dropped _array_element)))))
  (Utilities|IsValid _melee
    (:Is%20Valid
      (Actor|DestroyActor _melee)
      (return))
    (:Is%20Not%20Valid
      (return))))

(fn SelectedBestWeapon
  (Utilities|IsValid (Variables|Default|GetPrimary)
    (:Is%20Valid
      (if (CallFunction|CanEquippingWeapon "NewEnumerator0")
        (CallFunction|SelectedWeapon "NewEnumerator0")
        (else
          (CallFunction|SelectedWeapon "NewEnumerator2" :!label _label))))
    (:Is%20Not%20Valid
      (if (CallFunction|CanEquippingWeapon "NewEnumerator1")
        (Utilities|IsValid (Variables|Default|GetSecundary)
          (:Is%20Valid
            (CallFunction|SelectedWeapon "NewEnumerator1"))
          (:Is%20Not%20Valid
            (CallFunction|SelectedWeapon "NewEnumerator2")))
        (else
          (goto _label))))))