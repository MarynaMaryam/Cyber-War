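; Weapon Blueprint with swappable attachments (foregrip, light, dot sight, laser, silencer), each having first-person, third-person and UI widget components.
; SetPartMesh stores selections by part type and relays them through server and multicast RPCs.
; UpdatePartMeshes restores class-default attack data, then applies meshes, widget lists, sound overrides and socket attachments.
; Editor mode shows part widgets to the local owner, blocks attacks, and clears on casing, dropping or reloading.
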(event EventBeginPlay
  (|CallParentFunction)
  (Parts|UpdatePartMeshes))

(event Collision|EventActorBeginOverlap
  (params (OtherActor :type Actor%20Object%20Reference))
  (|CallParentFunction OtherActor) ; This node is disabled and will not be called.\nDrag off pins to build functionality.
)

(event EventTick
  (params (DeltaSeconds :type Float%20%28single-precision%29))
  (|CallParentFunction DeltaSeconds) ; This node is disabled and will not be called.\nDrag off pins to build functionality.
)

(event EventCaseWeapon
  (Variables|Parts|SetIsEditorMode false)
  (|CallParentFunction)
  (CallFunction|UpdateVisibility))

(event EventDropped
  (Variables|Parts|SetIsEditorMode false)
  (|CallParentFunction))

(event EventStartReloading
  (Variables|Parts|SetIsEditorMode false)
  (|CallParentFunction))

(event Custom|ServerSetEditorMode
  (params (IsEditorMode :type Boolean))
  (Variables|Parts|SetIsEditorMode IsEditorMode))

(event Custom|ServerSetPartMesh
  (params (Type :type EPartType%20Enum :default "NewEnumerator7") (ID :type Integer))
  (Parts|SetPartMesh Type ID))

(event Custom|MulticastSetPartMesh
  (params (Type :type EPartType%20Enum :default "NewEnumerator7") (ID :type Integer))
  (Networking|SwitchHasAuthority
    (:Remote
      (if (not (Pawn|IsLocallyControlled (CallFunction|GetPlayerOwner)))
        (Parts|SetPartMesh Type ID)))))

(fn ConstructionScript
  (|CallParentFunction))

(fn SetPartMesh
  (params (Type :type EPartType%20Enum :default "NewEnumerator7") (ID :type Integer))
  (Networking|SwitchHasAuthority
    (:Authority
      (CallFunction|MulticastSetPartMesh Type ID))
    (:Remote
      (CallFunction|ServerSetPartMesh Type ID)))
  (bind _result (Utilities|Set|ToArray (Variables|Parts|GetParts)))
  (for _array_element _result
    (if (Utilities|Enum|Equal(Enum) (.Type (Utilities|GetClassDefaults _array_element)) Type)
      (Utilities|Array|SetArrayElem (Variables|Parts|GetSelectedParts) (Math|Conversions|ToInteger(Byte) (.Type (Utilities|GetClassDefaults _array_element))) ID)))
  (Parts|UpdatePartMeshes)
  (return))

(fn SetEditorMode
  (params (IsEditorMode :type Boolean))
  (Networking|SwitchHasAuthority
    (:Authority
      _)
    (:Remote
      (CallFunction|ServerSetEditorMode IsEditorMode)))
  (Variables|Parts|SetIsEditorMode IsEditorMode)
  (CallFunction|UpdateVisibility)
  (return))

(fn CanStartAttack
  (params (Method :type EAttackMethod%20Enum :default "NewEnumerator0"))
  (return (and (|CallParentFunction Method) (not (Variables|Parts|GetIsEditorMode)))))

(fn IsEquippedPart
  (params (Type :type EPartType%20Enum :default "NewEnumerator7"))
  (return (> (Utilities|Array|Get(acopy) (Variables|Parts|GetSelectedParts) (Math|Conversions|ToInteger(Byte) Type)) -1)))

(fn UpdateVisibilityParts
  (params (bNewVisibility :type Boolean))
  (bind _foregripui (Variables|Default|GetForeGripUI))
  (Development|SetHiddeninGame _foregripui (Variables|Default|GetbHidden) false)
  (Utilities|IsValid (CallFunction|GetPlayerOwner)
    (:Is%20Valid
      (Rendering|SetVisibility _foregripui (and (Variables|Parts|GetIsEditorMode) (Pawn|IsLocallyControlled (CallFunction|GetPlayerOwner))) false)
      (Rendering|SetVisibility (Variables|Default|GetForeGrip1P) bNewVisibility false)
      (Class|PrimitiveComponent|SetOwnerNoSee (Variables|Default|GetForeGrip3P) bNewVisibility)
      (return))
    (:Is%20Not%20Valid
      (Rendering|SetVisibility (Variables|Default|GetDotSight1P) false true)
      (Class|PrimitiveComponent|SetOwnerNoSee (Variables|Default|GetDotSight3P) false)
      (return))))

(fn AttachmentParts
  (bind _result (Utilities|Set|ToArray (Variables|Parts|GetParts)))
  (for _array_element _result
    (Utilities|FlowControl|Sequence
      (:then_0
        (Utilities|IsValid (Utilities|Select :Index (.Type (Utilities|GetClassDefaults _array_element)) :NewEnumerator7 (Variables|Default|GetForeGrip1P) :NewEnumerator4 (Variables|Default|GetLight1P) :NewEnumerator5 (Variables|Default|GetDotSight1P) :NewEnumerator6 (Variables|Default|GetLaser1P) :NewEnumerator8 (Variables|Default|GetSilence1P))
          (:Is%20Valid
            (Transformation|AttachComponentToComponent (Utilities|Select :Index (.Type (Utilities|GetClassDefaults _array_element)) :NewEnumerator7 (Variables|Default|GetForeGrip1P) :NewEnumerator4 (Variables|Default|GetLight1P) :NewEnumerator5 (Variables|Default|GetDotSight1P) :NewEnumerator6 (Variables|Default|GetLaser1P) :NewEnumerator8 (Variables|Default|GetSilence1P)) (Variables|Default|GetWeaponMesh1P) (.Socket (Utilities|GetClassDefaults _array_element)) "SnapToTarget" "SnapToTarget" "SnapToTarget" true))))
      (:then_1
        (Utilities|IsValid (Utilities|Select :Index (.Type (Utilities|GetClassDefaults _array_element)) :NewEnumerator7 (Variables|Default|GetForeGrip3P) :NewEnumerator4 (Variables|Default|GetLight3P) :NewEnumerator5 (Variables|Default|GetDotSight3P) :NewEnumerator6 (Variables|Default|GetLaser3P) :NewEnumerator8 (Variables|Default|GetSilence3P))
          (:Is%20Valid
            (Transformation|AttachComponentToComponent (Utilities|Select :Index (.Type (Utilities|GetClassDefaults _array_element)) :NewEnumerator7 (Variables|Default|GetForeGrip3P) :NewEnumerator4 (Variables|Default|GetLight3P) :NewEnumerator5 (Variables|Default|GetDotSight3P) :NewEnumerator6 (Variables|Default|GetLaser3P) :NewEnumerator8 (Variables|Default|GetSilence3P)) (Variables|Default|GetWeaponMesh3P) (.Socket (Utilities|GetClassDefaults _array_element)) "SnapToTarget" "SnapToTarget" "SnapToTarget" true))))))
  (CallFunction|UpdateVisibility)
  (return))

(fn UpdatePartMeshes
  (Parts|UpdateDefaultsParameters)
  (bind _result (Utilities|Set|ToArray (Variables|Parts|GetParts)))
  (for _array_element _result
    (Utilities|FlowControl|Sequence
      (:then_0
        (Class|SkinnedMeshComponent|SetSkeletalMesh (Utilities|Select :Index (.Type (Utilities|GetClassDefaults _array_element)) :NewEnumerator7 (Variables|Default|GetForeGrip1P) :NewEnumerator4 (Variables|Default|GetLight1P) :NewEnumerator5 (Variables|Default|GetDotSight1P) :NewEnumerator6 (Variables|Default|GetLaser1P) :NewEnumerator8 (Variables|Default|GetSilence1P)) (.Mesh1P (Utilities|Struct|BreakFPartMeshInfo (Utilities|Array|Get(acopy) (.Meshes (Utilities|GetClassDefaults _array_element)) (Utilities|Array|Get(acopy) (Variables|Parts|GetSelectedParts) (Math|Conversions|ToInteger(Byte) (.Type (Utilities|GetClassDefaults _array_element))))))) true)
        (bind _aspart_mesh (Utilities|Casting|CastToPartMesh (UserInterface|GetUserWidgetObject (Utilities|Select :Index (.Type (Utilities|GetClassDefaults _array_element)) :NewEnumerator7 (Variables|Default|GetForeGripUI) :NewEnumerator4 (Variables|Default|GetLightUI) :NewEnumerator5 (Variables|Default|GetDotSightUI) :NewEnumerator6 (Variables|Default|GetLaserUI) :NewEnumerator8 (Variables|Default|GetSilenceUI)))))
        (Default|UpdatePartsList _aspart_mesh _array_element (Utilities|Array|Get(acopy) (Variables|Parts|GetSelectedParts) (Math|Conversions|ToInteger(Byte) (.Type (Utilities|GetClassDefaults _array_element))))))
      (:then_1
        (Class|SkinnedMeshComponent|SetSkeletalMesh (Utilities|Select :Index (.Type (Utilities|GetClassDefaults _array_element)) :NewEnumerator7 (Variables|Default|GetForeGrip3P) :NewEnumerator4 (Variables|Default|GetLight3P) :NewEnumerator5 (Variables|Default|GetDotSight3P) :NewEnumerator6 (Variables|Default|GetLaser3P) :NewEnumerator8 (Variables|Default|GetSilence3P)) (.Mesh3P (Utilities|Struct|BreakFPartMeshInfo (Utilities|Array|Get(acopy) (.Meshes (Utilities|GetClassDefaults _array_element)) (Utilities|Array|Get(acopy) (Variables|Parts|GetSelectedParts) (Math|Conversions|ToInteger(Byte) (.Type (Utilities|GetClassDefaults _array_element))))))) true))
      (:then_2
        (Parts|OverrideParameters (.Parameters (Utilities|Struct|BreakFPartMeshInfo (Utilities|Array|Get(acopy) (.Meshes (Utilities|GetClassDefaults _array_element)) (Utilities|Array|Get(acopy) (Variables|Parts|GetSelectedParts) (Math|Conversions|ToInteger(Byte) (.Type (Utilities|GetClassDefaults _array_element)))))))))))
  (Parts|AttachmentParts)
  (return))

(fn UpdateVisibility
  (bind _returnvalue (|CallParentFunction))
  (Parts|UpdateVisibilityParts _returnvalue)
  (return _returnvalue))

(fn OverrideParameters
  (params (PartsParameters :type F%20Parts%20Parameters%20Structure))
  (bind _sound (Utilities|Struct|BreakFPartsParameters PartsParameters))
  (bind _keys (Utilities|Map|Keys _sound))
  (for _array_element _keys
    (switch name _array_element
      (:BaseAttack
        (Variables|Default|SetAnimationBaseAttack (Utilities|Struct|MakeFAnimationWeapons (.Anim (Utilities|Struct|BreakFAnimationWeapons (Variables|Default|GetAnimationBaseAttack))) (.Arms (Utilities|Struct|BreakFAnimationWeapons (Variables|Default|GetAnimationBaseAttack))) (.Value (Utilities|Map|Find _sound _array_element))))))))

(fn UpdateDefaultsParameters
  (Variables|Default|SetAnimationBaseAttack (Utilities|GetClassDefaults (Utilities|GetClass self))))