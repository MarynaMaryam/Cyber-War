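; Weapon projectile that shows a muzzle effect on spawn and hands impacts back to its owning Weapon.
; On authority BeginPlay spawns muzzle particles on the 1P or 3P mesh and traces from the instigator's camera along control rotation.
; A trace hit on either of two special surface types stops the projectile immediately and applies weapon damage.
; Movement stop triggers the weapon's impact and a short lifespan; SpawnSoundProjectile is defined but uncalled here.
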(event OnProjectileStop(ProjectileMovement)
  (params (ImpactResult :type Hit%20Result%20Structure%20%28by%20ref%29))
  (bind _weapon (Variables|Components|GetWeapon))
  (Utilities|IsValid _weapon
    (:Is%20Valid
      (Default|SpawnImpact _weapon ImpactResult))
    (:Is%20Not%20Valid
      _))
  (Actor|SetLifeSpan 0.1))

(event Custom|SpawnParticalProjectile
  (params (Weapon :type Weapon%20Object%20Reference))
  (bind _muzzle (Variables|Effects|GetMuzzle))
  (bind _weaponmesh1p (Variables|/Game/Blueprints/Weapon/Weapon.Weapon_C|GetWeaponMesh1P Weapon))
  (bind _weaponmesh3p (Variables|/Game/Blueprints/Weapon/Weapon.Weapon_C|GetWeaponMesh3P Weapon))
  (if (CallFunction|IsNotDedicatedServer)
    (Utilities|IsValid Weapon
      (:Is%20Valid
        (if (Pawn|IsLocallyControlled (Default|GetPlayerOwner Weapon))
          (Effects|SpawnEmitterAttached _muzzle (Variables|/Game/Blueprints/Weapon/Weapon.Weapon_C|GetWeaponMesh1P Weapon) "Muzzle" (Transformation|GetSocketLocation _weaponmesh1p "Muzzle") (Transformation|GetSocketRotation _weaponmesh1p "Muzzle") "1.000000,1.000000,1.000000" "KeepWorldPosition")
          (else
            (Effects|SpawnEmitterAttached _muzzle (Variables|/Game/Blueprints/Weapon/Weapon.Weapon_C|GetWeaponMesh3P Weapon) "Muzzle" (Transformation|GetSocketLocation _weaponmesh3p "Muzzle") (Transformation|GetSocketRotation _weaponmesh3p "Muzzle") "1.000000,1.000000,1.000000" "KeepWorldPosition")))))))

(event EventBeginPlay
  (Networking|SwitchHasAuthority
    (:Authority
      (CallFunction|SpawnParticalProjectile (Variables|Components|GetWeapon))
      (CallFunction|CheckforObstacle))))

(event EventTick
  (params (DeltaSeconds :type Float%20%28single-precision%29)))

(fn ConstructionScript)

(fn SpawnSoundProjectile
  (bind _weapon (Variables|Components|GetWeapon))
  (Utilities|IsValid _weapon
    (:Is%20Valid
      (if (Pawn|IsLocallyControlled (Default|GetPlayerOwner _weapon))
        (return)
        (else
          (Audio|SpawnSoundAttached (Variables|Effects|GetMuzzleSound) (Variables|/Game/Blueprints/Weapon/Weapon.Weapon_C|GetWeaponMesh3P _weapon))
          (return))))))

(fn CheckforObstacle
  (bind _returnvalue (Game|GetInstigator))
  (bind _ascw_character (Utilities|Casting|CastToCW_Character _returnvalue))
  (bind _camera1p (Variables|/Game/Blueprints/Character/CW_Character.CW_Character_C|GetCamera1P _ascw_character))
  (bind _returnvalue_2 (Transformation|GetWorldLocation _camera1p))
  (bind (_outhit _returnvalue_3) (Collision|LineTraceByChannel _returnvalue_2 (+ _returnvalue_2 (* (Math|Vector|GetForwardVector (Pawn|GetControlRotation (Pawn|GetController _returnvalue) :!class /Script/Engine.Controller)) 1e+04)) "TraceTypeQuery3" true (Utilities|Array|MakeArray (Components|GetOwner) (Variables|Components|GetWeapon)) "ForDuration"))
  (if _returnvalue_3
    (if (or (Utilities|Enum|Equal(Enum) (Variables|/Script/Engine.PhysicalMaterial|GetSurfaceType (.PhysMat (Collision|BreakHitResult _outhit))) "SurfaceType24") (Utilities|Enum|Equal(Enum) (Variables|/Script/Engine.PhysicalMaterial|GetSurfaceType (.PhysMat (Collision|BreakHitResult _outhit))) "SurfaceType23"))
      (Game|Components|ProjectileMovement|StopSimulating (Variables|Default|GetProjectileMovement) _outhit)
      (Default|ApplyDamage (Variables|Components|GetWeapon) "NewEnumerator0" _outhit)
      (return)
      (else
        (return)))
    (else
      (return))))