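; Weapon inventory component for CW_Character that manages slot-based weapons, spawning PlayerState loadouts and handling equip, drop, override and overlap pickup.
; Attack, reload and editor-mode calls forward to the equipped weapon.
; RepNotifies drive equip and holster on the weapons and fall back to the best remaining one when Primary or Secundary empties.
; Pickup and drop go through multicast events, with pickup limited to empty Primary or Secundary slots.
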(event Custom|OnPlayerOverlap
  (params (OverlappedComponent :type Primitive%20Component%20Object%20Reference) (OtherActor :type Actor%20Object%20Reference) (OtherComp :type Primitive%20Component%20Object%20Reference) (OtherBodyIndex :type Integer) (bFromSweep :type Boolean) (SweepResult :type Hit%20Result%20Structure%20%28by%20ref%29))
  (CallFunction|HandleRaise OtherActor))

(event EventBeginPlay
  (bind _ascw_character (Utilities|Casting|CastToCW_Character (Components|GetOwner)))
  (Variables|Default|SetPlayerOwner _ascw_character)
  (Collision|BindEventtoOnComponentBeginOverlap (Variables|/Script/Engine.Character|GetCapsuleComponent (Variables|Default|GetPlayerOwner)) (delegate Custom|OnPlayerOverlap)))

(event EventTick
  (params (DeltaSeconds :type Float%20%28single-precision%29)))

(event Custom|HandleRaise
  (params (Actor :type Actor%20Object%20Reference))
  (bind _asweapon (Utilities|Casting|CastToWeapon Actor))
  (if (Utilities|DoesObjectImplementInterface Actor "/Game/Blueprints/Interface/IE_Interact.IE_Interact_C")
    (if (CallFunction|CanRaiseWeapon (Variables|/Game/Blueprints/Weapon/Weapon.Weapon_C|GetWeaponSlot _asweapon))
      (CallFunction|MulticastRaise _asweapon)
      (Default|SetOwnerWeapon _asweapon (Variables|Default|GetPlayerOwner)))))

(event Custom|BaseAttack
  (params (Activated :type Boolean))
  (bind _weapon (CallFunction|GetWeaponSelected))
  (Utilities|IsValid _weapon
    (:Is%20Valid
      (Default|StartAttack _weapon Activated "NewEnumerator0"))))

(event Custom|AdvancedAttack
  (params (Activated :type Boolean))
  (bind _weapon (CallFunction|GetWeaponSelected))
  (Utilities|IsValid _weapon
    (:Is%20Valid
      (Default|StartAttack _weapon Activated "NewEnumerator1"))))

(event Custom|Reloading
  (bind _weapon (CallFunction|GetWeaponSelected))
  (Utilities|IsValid _weapon
    (:Is%20Valid
      (Default|StartReloading _weapon))))

(event Custom|MulticastRaise
  (params (Actor :type Actor%20Object%20Reference))
  (Class|IEInteract|Interact(Message) Actor (Components|GetOwner)))

(event Custom|MulticastDropped
  (params (Weapon :type Weapon%20Object%20Reference))
  (Default|Dropped Weapon))

(fn SpawnWeapon
  (params (Weapon :type Weapon%20Class%20Reference))
  (bind _returnvalue (Components|GetOwner))
  (Utilities|IsValidClass Weapon
    (:Is%20Valid
      (bind _returnvalue_2 (Game|SpawnActorfromClass Weapon (Transformation|GetActorTransform _returnvalue) "AlwaysSpawn" _returnvalue 0))
      (Default|SetOwnerWeapon _returnvalue_2 _returnvalue)
      (return))
    (:Is%20Not%20Valid
      (return))))

(fn GetWeaponSelected
  (return (Variables|Default|GetEquipping)))

(fn SetWeapon
  (params (Slot :type EWeaponSlot%20Enum :default "NewEnumerator0") (Weapon :type Weapon%20Object%20Reference))
  (LocalVariables|SetLocalWeapon Weapon)
  (switch Utilities|FlowControl|Switch|SwitchonEWeaponSlot Slot
    (:NewEnumerator0
      (Variables|Default|SetPrimary (LocalVariables|GetLocalWeapon)))
    (:NewEnumerator1
      (Variables|Default|SetSecundary (LocalVariables|GetLocalWeapon)))
    (:NewEnumerator2
      (Variables|Default|SetMelee (LocalVariables|GetLocalWeapon)))
    (:NewEnumerator3
      (Variables|Default|SetThrow (LocalVariables|GetLocalWeapon)))
    (:NewEnumerator4
      (Variables|Default|SetSpecial (LocalVariables|GetLocalWeapon)))))

(fn SelectedWeapon
  (params (Slot :type EWeaponSlot%20Enum :default "NewEnumerator0"))
  (if (CallFunction|CanEquippingWeapon Slot)
    (Utilities|IsValid (Variables|Default|GetEquipping)
      (:Is%20Valid
        (Variables|Default|SetLastWeapon (Variables|Default|GetEquipping)))
      (:Is%20Not%20Valid
        _))
    (Variables|Default|SetEquipping (CallFunction|GetWeapon Slot))
    (return)
    (else
      (return))))

(fn CanEquippingWeapon
  (params (Slot :type EWeaponSlot%20Enum :default "NewEnumerator0"))
  (bind _equipping (Variables|Default|GetEquipping))
  (Utilities|IsValid _equipping
    (:Is%20Valid
      (return (and (Utilities|Enum|NotEqual(Enum) Slot (Variables|/Game/Blueprints/Weapon/Weapon.Weapon_C|GetWeaponSlot _equipping)) (Utilities|IsValid (CallFunction|GetWeapon Slot)))))
    (:Is%20Not%20Valid
      (return true))))

(fn GetWeapon
  (params (Slot :type EWeaponSlot%20Enum%20%28by%20ref%29 :default "NewEnumerator0"))
  (return (Utilities|Select :Index Slot :NewEnumerator0 (Variables|Default|GetPrimary) :NewEnumerator1 (Variables|Default|GetSecundary) :NewEnumerator2 (Variables|Default|GetMelee) :NewEnumerator3 (Variables|Default|GetThrow) :NewEnumerator4 (Variables|Default|GetSpecial))))

(fn SpawnDefaultWeapons
  (params (PlayerState :type Player%20State%20Object%20Reference))
  (Utilities|IsValid PlayerState
    (:Is%20Valid
      (bind _ascw_player_state (Utilities|Casting|CastToCW_PlayerState PlayerState))
      (for _array_element (Utilities|Array|MakeArray (Default|GetSelectedWeapon _ascw_player_state "NewEnumerator0") (Default|GetSelectedWeapon _ascw_player_state "NewEnumerator1") (Default|GetSelectedWeapon _ascw_player_state "NewEnumerator2"))
        (CallFunction|SpawnWeapon _array_element))
      (CallFunction|SelectedWeapon (CallFunction|GetBestWeapon))
      (return))))

(fn OnRepEquipping
  (bind _equipping (Variables|Default|GetEquipping))
  (Utilities|IsValid _equipping
    (:Is%20Valid
      (Default|SelectedWeapon _equipping)
      (return))
    (:Is%20Not%20Valid
      (return))))

(fn OnRepPrimary
  (Utilities|IsValid (Variables|Default|GetPrimary)
    (:Is%20Valid
      (return))
    (:Is%20Not%20Valid
      (CallFunction|SelectedWeapon (CallFunction|GetBestWeapon))
      (return))))

(fn OnRepSecundary
  (Utilities|IsValid (Variables|Default|GetSecundary)
    (:Is%20Valid
      (return))
    (:Is%20Not%20Valid
      (CallFunction|SelectedWeapon (CallFunction|GetBestWeapon))
      (return))))

(fn OnRepMelee
  (bind _melee (Variables|Default|GetMelee))
  (Utilities|IsValid _melee
    (:Is%20Valid
      (Default|SetOwnerWeapon _melee (Components|GetOwner))
      (return))
    (:Is%20Not%20Valid
      (return))))

(fn OnRepThrow)

(fn OnRepSpecial)

(fn OnRepLastWeapon
  (bind _lastweapon (Variables|Default|GetLastWeapon))
  (Utilities|IsValid _lastweapon
    (:Is%20Valid
      (if (!= (Components|GetOwner _lastweapon) (Components|GetOwner))
        (return)
        (else
          (Default|CaseWeapon _lastweapon)
          (return))))
    (:Is%20Not%20Valid
      (return))))

(fn DroppedWeapon
  (bind _equipping (Variables|Default|GetEquipping))
  (Utilities|IsValid _equipping
    (:Is%20Valid
      (if (Default|CanDroppedWeapon _equipping)
        (CallFunction|MulticastDropped _equipping)
        (CallFunction|SetWeapon (Variables|/Game/Blueprints/Weapon/Weapon.Weapon_C|GetWeaponSlot _equipping))
        (else
          (return))))
    (:Is%20Not%20Valid
      (return))))

(fn CanRaiseWeapon
  (params (Slot :type EWeaponSlot%20Enum :default "NewEnumerator0"))
  (switch Utilities|FlowControl|Switch|SwitchonEWeaponSlot Slot
    (:NewEnumerator0
      (Variables|Default|GetPrimary
        (:then
          _)
        (:else
          (return true))))
    (:NewEnumerator1
      (Variables|Default|GetSecundary
        (:then
          _)
        (:else
          (return true))))
    (:NewEnumerator2
      (return false)))
  (return false))

(fn DestroyAllWeapons
  (for _array_element (Utilities|Array|MakeArray (Variables|Default|GetPrimary) (Variables|Default|GetSecundary) (Variables|Default|GetMelee))
    (Utilities|IsValid _array_element
      (:Is%20Valid
        (Actor|DestroyActor _array_element))))
  (return))

(fn GetBestWeapon
  (Utilities|IsValid (Variables|Default|GetPrimary)
    (:Is%20Valid
      (return "NewEnumerator0"))
    (:Is%20Not%20Valid
      (Utilities|IsValid (Variables|Default|GetSecundary)
        (:Is%20Valid
          (return "NewEnumerator1"))
        (:Is%20Not%20Valid
          (return "NewEnumerator2"))))))

(fn EditorMode
  (bind _weapon (CallFunction|GetWeaponSelected))
  (Utilities|IsValid _weapon
    (:Is%20Valid
      (bind _asweap_parts (Utilities|Casting|CastToWeapParts _weapon))
      (Default|SetEditorMode _asweap_parts (not (Variables|/Game/Blueprints/Weapon/WeapParts.WeapParts_C|GetIsEditorMode _asweap_parts))))))

(fn OverrideSelecterWeapon
  (params (Slot :type EWeaponSlot%20Enum :default "NewEnumerator0") (Weapon :type Weapon%20Class%20Reference))
  (bind _weapon (CallFunction|GetWeapon Slot))
  (if (CallFunction|CanOverrideWeapon Slot Weapon)
    (Utilities|IsValid _weapon
      (:Is%20Valid
        (Actor|DestroyActor _weapon))
      (:Is%20Not%20Valid
        _))
    (CallFunction|SpawnWeapon Weapon)
    (CallFunction|SelectedWeapon Slot)
    (return)))

(fn CanOverrideWeapon
  (params (Slot :type EWeaponSlot%20Enum%20%28by%20ref%29 :default "NewEnumerator0") (Weapon :type Weapon%20Class%20Reference))
  (return (!= (Utilities|GetClass (CallFunction|GetWeapon Slot)) Weapon)))