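; Weapon projectile Blueprint that handles muzzle effects, obstacle hits and impacts for the weapon that fired it.
; On authority at BeginPlay, it triggers muzzle effects for non-dedicated instances, choosing first- or third-person mesh and silencer socket, with sound for non-local shooters.
; It also traces forward, immediately stopping and applying weapon damage on two specific surface types.
; When movement stops, the weapon spawns the impact and the projectile expires shortly after.
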(event OnProjectileStop(ProjectileMovement)
  (params (ImpactResult :type Hit%20Result%20Structure%20%28by%20ref%29))
  (bind _weapon (Variables|Components|GetWeapon))
  (Utilities|IsValid _weapon
    (:Is%20Valid
      (Default|SpawnImpact _weapon ImpactResult))
    (:Is%20Not%20Valid
      _))
  (Actor|SetLifeSpan 0.1))

(event Custom|SpawnParticalProjectile
  (params (Weapon :type Weapon%20Object%20Reference))
  (bind _currentowner (Default|GetPlayerOwner Weapon))
  (bind _weaponmesh1p (Variables|/Game/Blueprints/Weapon/Weapon.Weapon_C|GetWeaponMesh1P Weapon))
  (bind _weaponmesh3p (Variables|/Game/Blueprints/Weapon/Weapon.Weapon_C|GetWeaponMesh3P Weapon))
  (bind _muzzle (Variables|Effects|GetMuzzle))
  (bind _returnvalue (Default|IsThirdPerson _currentowner))
  (bind _returnvalue_2 (Pawn|IsLocallyControlled _currentowner))
  (bind _returnvalue_3 (not _returnvalue))
  (bind _returnvalue_4 (and _returnvalue_2 _returnvalue_3))
  (if (CallFunction|IsNotDedicatedServer)
    (Utilities|IsValid Weapon
      (:Is%20Valid
        (CallFunction|SpawnMuzzleSound)
        (bind _asweap_parts (Utilities|Casting|CastToWeapParts Weapon)
          (:then
            (if _returnvalue_4
              (Effects|SpawnEmitterAttached _muzzle _weaponmesh1p (select (Default|IsEquippedPart _asweap_parts "NewEnumerator8") "MuzzleSilence" "Muzzle") "0, 0, 0" "0, 0, 0" "1.000000,1.000000,1.000000" "SnapToTarget")
              (else
                (Effects|SpawnEmitterAttached _muzzle _weaponmesh3p (select (Default|IsEquippedPart _asweap_parts "NewEnumerator8") "MuzzleSilence" "Muzzle") "0, 0, 0" "0, 0, 0" "1.000000,1.000000,1.000000" "SnapToTarget"))))
          (:CastFailed
            (if _returnvalue_4
              (Effects|SpawnEmitterAttached _muzzle _weaponmesh1p "Muzzle" "0, 0, 0" "0, 0, 0" "1.000000,1.000000,1.000000" "SnapToTarget")
              (else
                (Effects|SpawnEmitterAttached _muzzle _weaponmesh3p "Muzzle" (select (.bSuccess (Utilities|Casting|CastToWeap_Anaconda Weapon)) "24.500000, 0,1.500000" "0, 0, 0") "0, 0, 0" "1.000000,1.000000,1.000000" "SnapToTarget")))))))))

(event EventBeginPlay
  (Networking|SwitchHasAuthority
    (:Authority
      (CallFunction|SpawnParticalProjectile (Variables|Components|GetWeapon))
      (CallFunction|CheckforObstacle))))

(event EventTick
  (params (DeltaSeconds :type Float%20%28single-precision%29)))

(fn ConstructionScript)

(fn CheckforObstacle
  (bind _returnvalue (Transformation|GetActorLocation))
  (bind (_outhit _returnvalue_2) (Collision|LineTraceByChannel _returnvalue (+ _returnvalue (* (Math|Vector|GetForwardVector (Transformation|GetActorRotation)) 1e+04)) "TraceTypeQuery3" true (Utilities|Array|MakeArray (Components|GetOwner) (Variables|Components|GetWeapon)) "ForDuration"))
  (if _returnvalue_2
    (if (or (Utilities|Enum|Equal(Enum) (Variables|/Script/Engine.PhysicalMaterial|GetSurfaceType (.PhysMat (Collision|BreakHitResult _outhit))) "SurfaceType24") (Utilities|Enum|Equal(Enum) (Variables|/Script/Engine.PhysicalMaterial|GetSurfaceType (.PhysMat (Collision|BreakHitResult _outhit))) "SurfaceType23"))
      (Game|Components|ProjectileMovement|StopSimulating (Variables|Default|GetProjectileMovement) _outhit)
      (Default|ApplyDamage (Variables|Components|GetWeapon) "NewEnumerator0" _outhit)
      (return)
      (else
        (return)))
    (else
      (return))))

(fn SpawnMuzzleSound
  (bind _weapon (Variables|Components|GetWeapon))
  (Utilities|IsValid _weapon
    (:Is%20Valid
      (if (not (Pawn|IsLocallyControlled (Default|GetPlayerOwner _weapon)))
        (Audio|SpawnSoundAttached (.Sound (Utilities|Struct|BreakFAnimationWeapons (Variables|/Game/Blueprints/Weapon/Weapon.Weapon_C|GetAnimationBaseAttack _weapon))) (Variables|/Game/Blueprints/Weapon/Weapon.Weapon_C|GetWeaponMesh1P _weapon) "Muzzle" "0, 0, 0" "0, 0, 0" "SnapToTarget")))))