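; Lobby game mode for online play that holds off starting the match until the game instance triggers player creation.
; On BeginPlay it hands its CreatePlayer event to CW_GameInstance as a callback, and that event calls StartMatch.
; A SpawnCharacter helper, not called within this Blueprint, spawns a CW_Character at the first PlayerStart found, adjusting for collisions.
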(event Custom|CreatePlayer
  (Class|GameMode|StartMatch))

(event EventBeginPlay
  (bind _ascw_game_instance (Utilities|Casting|CastToCW_GameInstance (Game|GetGameInstance)))
  (EventDispatchers|AssignCreatePlayer _ascw_game_instance (delegate Custom|CreatePlayer)))

(event EventTick
  (params (DeltaSeconds :type Float%20%28single-precision%29)))

(fn ConstructionScript)

(fn SpawnCharacter
  (Game|SpawnActorfromClass "/Game/Blueprints/Character/CW_Character.CW_Character_C" (CallFunction|GetTransformSpawn) "AdjustIfPossibleButDontSpawnIfColliding" 0 0))

(fn GetTransformSpawn
  (bind _outactors (Actor|GetAllActorsOfClass "/Script/Engine.PlayerStart"))
  (Utilities|IsValid (Utilities|Array|Get(acopy) _outactors)
    (:Is%20Valid
      (return (Transformation|GetActorTransform (Utilities|Array|Get(acopy) _outactors))))
    (:Is%20Not%20Valid
      (return ""))))