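; CW_HUD is the player HUD that opens a UI page through CW_GameInstance and maintains the character and weapon values for display.
; Every DrawHUD frame it polls the owning CW_Character, caching health text, plus ammo text and visibility from the WeaponManager's selected weapon, hiding ammo when infinite.
; It also mirrors the editor-mode flag of WeapParts weapons and toggles the mouse cursor to match.
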(event EventBeginPlay
  (bind _ascw_game_instance (Utilities|Casting|CastToCW_GameInstance (Game|GetGameInstance)))
  (Default|ShowPage _ascw_game_instance false "NewEnumerator6" (Game|Player|GetOwningPlayerController)))

(event EventDrawHUD
  (params (SizeX :type Integer) (SizeY :type Integer))
  (CallFunction|UpdateCharacterData)
  (CallFunction|UpdateWeaponData)
  (CallFunction|UpdateEditorWeapon))

(fn ConstructionScript)

(fn UpdateCharacterData
  (bind _returnvalue (Class|HUD|GetOwningPawn))
  (bind _ascw_character (Utilities|Casting|CastToCW_Character _returnvalue))
  (Utilities|FlowControl|Sequence
    (:then_0
      (if (!= _ascw_character (Variables|Default|GetCharacter))
        (Variables|Default|SetCharacter _ascw_character)))
    (:then_1
      (Utilities|IsValid (Variables|Default|GetCharacter)
        (:Is%20Valid
          (Variables|Default|SetDisplayHealth (Utilities|String|ToString(Integer) (Math|Float|Floor (Variables|/Game/Blueprints/Character/CW_Character.CW_Character_C|GetHealth (Variables|Default|GetCharacter))))))
        (:Is%20Not%20Valid
          (Variables|Default|SetDisplayHealth "-"))))
    (:then_2
      (return))))

(fn UpdateWeaponData
  (bind _character (Variables|Default|GetCharacter))
  (bind _weaponmanager (Variables|/Game/Blueprints/Character/CW_Character.CW_Character_C|GetWeaponManager _character))
  (bind _weapon (Default|GetWeaponSelected _weaponmanager))
  (Utilities|IsValid _weapon
    (:Is%20Valid
      (Variables|Default|SetVisibilityAmmo (select (Variables|/Game/Blueprints/Weapon/Weapon.Weapon_C|GetInfiniteAmmo _weapon) "Hidden" "Visible"))
      (Variables|Default|SetDisplayAmmo (Utilities|String|Append (Utilities|String|ToString(Integer) (Variables|/Game/Blueprints/Weapon/Weapon.Weapon_C|GetMagazineAmmo _weapon)) "/" (Utilities|String|ToString(Integer) (Variables|/Game/Blueprints/Weapon/Weapon.Weapon_C|GetTotalAmmo _weapon))))
      (return))))

(fn UpdateEditorWeapon
  (bind _returnvalue (Game|Player|GetOwningPlayerController))
  (bind _character (Variables|Default|GetCharacter)
    (:then
      (bind _weaponmanager (Variables|/Game/Blueprints/Character/CW_Character.CW_Character_C|GetWeaponManager _character)
        (:then
          (Utilities|IsValid (Default|GetWeaponSelected _weaponmanager)
            (:Is%20Valid
              (bind _asweap_parts (Utilities|Casting|CastToWeapParts (Default|GetWeaponSelected _weaponmanager))
                (:then
                  (Variables|Default|SetIsEditorMode (Variables|/Game/Blueprints/Weapon/WeapParts.WeapParts_C|GetIsEditorMode _asweap_parts))
                  (Variables|/Script/Engine.PlayerController|SetbShowMouseCursor _returnvalue (Variables|/Game/Blueprints/Weapon/WeapParts.WeapParts_C|GetIsEditorMode _asweap_parts)))
                (:CastFailed
                  (Variables|Default|SetIsEditorMode false)
                  (Variables|/Script/Engine.PlayerController|SetbShowMouseCursor _returnvalue false))))))
        (:else)))
    (:else)))