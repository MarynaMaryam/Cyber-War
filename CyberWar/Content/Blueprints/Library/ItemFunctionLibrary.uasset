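; Blueprint function library for looking up items in the ItemTable data table and converting their assets.
; Row names double as integer IDs: GetItem fetches one row by ID, and GetAllItems builds an ID-to-item map.
; GetItemId reverse-looks up an ID by matching Asset across that map, returning -1 on no match.
; Helpers cast an item's Asset to CW_CharacterMesh or Weapon, or construct an object from a class.
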(fn GetAllItems
  (bind _outrownames (DataTable|GetDataTableRowNames "/Game/Blueprints/Game/ItemTable.ItemTable"))
  (for _array_element _outrownames
    (bind _returnvalue (Utilities|GetDataTableRow "/Game/Blueprints/Game/ItemTable.ItemTable" _array_element)
      (:then
        (Utilities|Map|Add (LocalVariables|GetLocalArrayItems) (Math|Conversions|ToInteger(Byte) (Utilities|String|ToString(Name) _array_element)) _returnvalue))))
  (return (LocalVariables|GetLocalArrayItems)))

(fn GetItem
  (params (ItemId :type Integer))
  (bind _returnvalue (Utilities|GetDataTableRow "/Game/Blueprints/Game/ItemTable.ItemTable" (Utilities|String|StringToName (Utilities|String|ToString(Integer) ItemId)))
    (:then
      (return _returnvalue))
    (:RowNotFound
      (return ""))))

(fn ItemtoCharacterMesh
  (params (Item :type F%20Item%20Data%20Structure))
  (bind _ascw_character_mesh (Utilities|Casting|CastToCW_CharacterMeshClass (.Asset (Utilities|Struct|BreakFItemData Item)))
    (:then
      (return _ascw_character_mesh))
    (:CastFailed
      (return 0))))

(fn ItemtoWeapon
  (params (Item :type F%20Item%20Data%20Structure))
  (bind _asweapon (Utilities|Casting|CastToWeaponClass (.Asset (Utilities|Struct|BreakFItemData Item)))
    (:then
      (return _asweapon))
    (:CastFailed
      (return 0))))

(fn ClasstoObject
  (params (Class :type CW%20Character%20Mesh%20Class%20Reference))
  (bind _returnvalue (Game|ConstructObjectfromClass Class (LocalVariables|Get__WorldContext)))
  (return _returnvalue))

(fn GetItemId
  (params (Item :type F%20Item%20Data%20Structure))
  (bind ___worldcontext (LocalVariables|Get__WorldContext))
  (bind _items (Game|Items|GetAllItems ___worldcontext))
  (bind _values (Utilities|Map|Values _items))
  (for (_array_element _array_index) _values
    (if (== (.asset _array_element) (.Asset (Utilities|Struct|BreakFItemData Item)))
      (bind _keys (Utilities|Map|Keys _items))
      (return (Utilities|Array|Get(acopy) _keys _array_index))))
  (return -1))