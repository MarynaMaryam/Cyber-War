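; Blueprint function library of shared helpers for level, network, logging, hit-location and player data queries.
; It checks for the "Lobby" level and non-dedicated servers, and prints log-only, timestamped messages with color and duration chosen by log type.
; DefinitionDamageType maps Bip 001 skeleton bone names to head, torso, arm, leg or default damage types.
; GetPlayerMetadata returns the metadata stored on CW_GameInstance when valid.
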(fn IsCurrentLevelLobby
  (bind _returnvalue (Game|GetCurrentLevelName (LocalVariables|Get__WorldContext)))
  (return (Utilities|Enum|Equal(Enum) _returnvalue "Lobby")))

(fn PrintLog
  (params (Text :type Text) (LogType :type ELogType%20Enum :default "NewEnumerator0"))
  (bind _returnvalue (Math|DateTime|Now))
  (bind ___worldcontext (LocalVariables|Get__WorldContext))
  (bind (_year _month _day _hour _minute _second _millisecond) (Math|DateTime|BreakDateTime _returnvalue))
  (Development|PrintText ___worldcontext (Utilities|Text|FormatText "{WorldContext}( {Time} ) - {TextLog}" (select (Networking|IsNotDedicatedServer ___worldcontext) (Utilities|Text|FormatText "[ {Text} ]: " (Utilities|Text|ToText(String) (Utilities|GetObjectName ___worldcontext))) ":") (Utilities|Text|FormatText "{Second}:{Millisecond}" _second _millisecond) Text) false true (Utilities|Select :Index LogType :NewEnumerator0 "(R=0.000000,G=1.000000,B=0.000000,A=1.000000)" :NewEnumerator1 "(R=1.000000,G=1.000000,B=0.000000,A=1.000000)" :NewEnumerator2 "(R=1.000000,G=0.000000,B=0.000000,A=1.000000)" :NewEnumerator3 "(R=0.000000,G=0.272204,B=1.000000,A=1.000000)") (Utilities|Select :Index LogType :NewEnumerator0 1e+01 :NewEnumerator1 15.0 :NewEnumerator2 2e+01 :NewEnumerator3 5.0)))

(fn IsNotDedicatedServer
  (return (not (Networking|IsDedicatedServer (LocalVariables|Get__WorldContext)))))

(fn DefinitionDamageType
  (params (Selection :type Name))
  (switch name Selection
    (:Default
      (bind _output_get (LocalVariables|SetDamageType "NewEnumerator4"))
      (return _output_get))
    (:Bip001-Head1
      (bind _output_get_2 (LocalVariables|SetDamageType "NewEnumerator0"))
      (return _output_get_2))
    (:Bip001-Spine001
      _)
    (:Bip001-Spine003
      _)
    (:Bip001-Pelvis001
      _)
    (:Bip001-R-Thigh001
      (bind _output_get_3 (LocalVariables|SetDamageType "NewEnumerator3" :!label _label))
      (return _output_get_3))
    (:Bip001-R-Calf001
      (goto _label))
    (:Bip001-R-Foot001
      (goto _label))
    (:Bip001-L-Thigh001
      (goto _label))
    (:Bip001-L-Calf001
      (goto _label))
    (:Bip001-L-Foot001
      (goto _label))
    (:Bip001-R-UpperArm001
      (bind _output_get_4 (LocalVariables|SetDamageType "NewEnumerator2" :!label _label_2))
      (return _output_get_4))
    (:Bip001-R-Forearm001
      (goto _label_2))
    (:Bip001-R-Hand001
      (goto _label_2))
    (:Bip001-L-UpperArm001
      (goto _label_2))
    (:Bip001-L-Forearm001
      (goto _label_2))
    (:Bip001-L-Hand001
      (goto _label_2)))
  (bind _output_get_5 (LocalVariables|SetDamageType "NewEnumerator1"))
  (return _output_get_5))

(fn GetPlayerMetadata
  (bind ___worldcontext (LocalVariables|Get__WorldContext))
  (bind _returnvalue (Game|GetGameInstance ___worldcontext))
  (bind _ascw_game_instance (Utilities|Casting|CastToCW_GameInstance _returnvalue))
  (bind _playermetadata (Variables|/Game/Blueprints/Engine/CW_GameInstance.CW_GameInstance_C|GetPlayerMetadata _ascw_game_instance))
  (Utilities|IsValid _playermetadata
    (:Is%20Valid
      (return _playermetadata))
    (:Is%20Not%20Valid
      (return 0))))