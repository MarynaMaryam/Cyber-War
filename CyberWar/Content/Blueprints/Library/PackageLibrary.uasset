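; Blueprint function library that converts network packages between bytes and JSON for socket communication with a server.
; BytesToPackage decodes UTF-8 bytes into a JSON object.
; PackageToBytes wraps an action string and data object in JSON, then, only if the socket is valid and connected, logs it and returns UTF-8 bytes.
; Otherwise it logs a Russian-language failure message and returns without encoding.
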(fn BytestoPackage
  (params (Bytes :type Array%20of%20Bytes))
  (LocalVariables|SetJson (Class|VaRestJsonObject|ConstructJsonObject))
  (Class|VaRestJsonObject|DecodeJson (LocalVariables|GetJson) (Class|LowEntryExtendedStandardLibrary|BytestoStringUtf8 Bytes))
  (return (LocalVariables|GetJson)))

(fn PackagetoBytes
  (params (Bytes :type F%20Package%20Structure%20%28by%20ref%29) (Socket :type Low%20Entry%20Socket%20Connection%20Object%20Reference%20%28by%20ref%29))
  (bind ___worldcontext (LocalVariables|Get__WorldContext))
  (LocalVariables|SetJson (Class|VaRestJsonObject|ConstructJsonObject))
  (Class|VaRestJsonObject|SetStringField (LocalVariables|GetJson) "action" (.action Bytes))
  (Class|VaRestJsonObject|SetObjectField (LocalVariables|GetJson) "data" (.data Bytes))
  (Utilities|IsValid Socket
    (:Is%20Valid
      (if (Class|LowEntrySocketConnection|IsConnected Socket)
        (CallFunction|PrintLog (Utilities|Text|FormatText "Send Package: {Package}" (Utilities|Text|ToText(String) (Class|VaRestJsonObject|EncodeJsontoSingleString (LocalVariables|GetJson)))) "NewEnumerator0" (LocalVariables|Get__WorldContext))
        (return (Class|LowEntryExtendedStandardLibrary|StringtoBytesUtf8 (Class|VaRestJsonObject|EncodeJsontoSingleString (LocalVariables|GetJson))))
        (else
          (CallFunction|PrintLog "Не удалось отправить пакет, соеденение с сервером не найдено." "NewEnumerator1" ___worldcontext)
          (return 0))))
    (:Is%20Not%20Valid
      (CallFunction|PrintLog "Не удалось отправить пакет, сокет не валидный." "NewEnumerator1" ___worldcontext)
      (return 0))))