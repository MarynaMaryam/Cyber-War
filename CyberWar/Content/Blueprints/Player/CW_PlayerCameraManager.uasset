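; Player camera manager that picks which camera drives the player's view through a BlueprintUpdateCamera override.
; For a CW_Character view target, it uses the lobby camera in lobby levels, otherwise the third- or first-person camera by the character's mode.
; For any other target, it falls back to a level CameraActor tagged "Default", found by searching all camera actors on each such update.
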(event EventBeginPlay)

(event Collision|EventActorBeginOverlap
  (params (OtherActor :type Actor%20Object%20Reference)))

(event EventTick
  (params (DeltaSeconds :type Float%20%28single-precision%29)))

(fn ConstructionScript)

(fn BlueprintUpdateCamera
  (params (CameraTarget :type Actor%20Object%20Reference))
  (bind _ascw_character (Utilities|Casting|CastToCW_Character CameraTarget)
    (:then
      (bind _desiredview (Class|CameraComponent|GetCameraView (select (CallFunction|IsCurrentLevelLobby) (Variables|/Game/Blueprints/Character/CW_Character.CW_Character_C|GetCameraLobby _ascw_character) (select (Default|IsThirdPerson _ascw_character) (Variables|/Game/Blueprints/Character/CW_Character.CW_Character_C|GetCamera3P _ascw_character) (Variables|/Game/Blueprints/Character/CW_Character.CW_Character_C|GetCamera1P _ascw_character))) (Utilities|Time|GetWorldDeltaSeconds)))
      (return (.location _desiredview) (.rotation _desiredview) (.fov _desiredview) true))
    (:CastFailed
      (bind _outactors (Actor|GetAllActorsOfClass "/Script/Engine.CameraActor"))
      (for _array_element _outactors
        (if (Actor|ActorHasTag _array_element "Default")
          (bind _desiredview_2 (Class|CameraComponent|GetCameraView (Variables|/Script/Engine.CameraActor|GetCameraComponent _array_element) (Utilities|Time|GetWorldDeltaSeconds)))
          (return (.location _desiredview_2) (.rotation _desiredview_2) (.fov _desiredview_2) true))))))