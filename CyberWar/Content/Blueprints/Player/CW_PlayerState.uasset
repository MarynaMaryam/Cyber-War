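; Player state that tracks a player's team, per-team character mesh selection, and death, ally-kill and rival-kill counts.
; The team chooses the Red or Blue selection as an item ID, which resolves to the character mesh.
; RepNotifies on team and both selections refresh the mesh through the owning controller's pawn.
; Without a CW_PlayerController owner, it searches all CW_Characters for the one referencing this state.
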(event EventBeginPlay)

(event EventTick
  (params (DeltaSeconds :type Float%20%28single-precision%29)))

(fn ConstructionScript)

(fn GetCharacterMeshID
  (return (Utilities|Select :Index (Variables|PlayerState|GetTeam) :NewEnumerator2 0 :NewEnumerator0 (Variables|PlayerState|GetSelectedCharacterMeshRed) :NewEnumerator1 (Variables|PlayerState|GetSelectedCharacterMeshBlue))))

(fn GetCharacterMesh
  (return (CallFunction|ItemtoCharacterMesh (CallFunction|GetItem (CallFunction|GetCharacterMeshID)))))

(fn UpdateCharacterMesh
  (bind _ascw_player_controller (Utilities|Casting|CastToCW_PlayerController (Components|GetOwner))
    (:then
      (bind _ascw_character (Utilities|Casting|CastToCW_Character (Pawn|GetControlledPawn _ascw_player_controller))
        (:then
          (Default|UpdateCharacterMesh _ascw_character))
        (:CastFailed
          (return))))
    (:CastFailed
      (bind _outactors (Actor|GetAllActorsOfClass "/Game/Blueprints/Character/CW_Character.CW_Character_C"))
      (bind _array_element (Utilities|Array|ForEachLoopwithBreak _outactors :!label _label)
        (:LoopBody
          (if (== (Variables|/Game/Blueprints/Character/CW_Character.CW_Character_C|GetCWPlayerState _array_element) self)
            (Default|UpdateCharacterMesh _array_element)
            (goto _label Break)))
        (:Completed
          (return))))))

(fn OnRepSelectedCharacterMeshRed
  (CallFunction|UpdateCharacterMesh)
  (return))

(fn OnRepSelectedCharacterMeshBlue
  (CallFunction|UpdateCharacterMesh)
  (return))

(fn OnRepTeam
  (CallFunction|UpdateCharacterMesh)
  (return))

(fn IncrementDeaths
  (Variables|PlayerState|SetDeaths (+ (Variables|PlayerState|GetDeaths) 1))
  (return))

(fn IncrementKills
  (params (bWasTeamKill :type Boolean))
  (if bWasTeamKill
    (Variables|PlayerState|SetAlliesKilled (+ (Variables|PlayerState|GetAlliesKilled) 1))
    (return)
    (else
      (Variables|PlayerState|SetRivalsKilled (+ (Variables|PlayerState|GetRivalsKilled) 1))
      (return))))